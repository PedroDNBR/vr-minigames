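; Test actor whose mesh is cut in two when a GrippableStaticMeshActor hits it.
; The construction script copies the StaticMesh component into a ProceduralMesh with collision.
; On hit, it slices that mesh at the hit location with a capped cut, enables physics on the new half and applies an impulse scaled from the impact point to both halves.
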(event OnComponentHit(ProceduralMesh)
  (params (HitComponent :type Primitive%20Component%20Object%20Reference) (OtherActor :type Actor%20Object%20Reference) (OtherComp :type Primitive%20Component%20Object%20Reference) (NormalImpulse :type Vector :default "0, 0, 0") (Hit :type Hit%20Result%20Structure%20%28by%20ref%29))
  (bind (_bblockinghit _binitialoverlap _time _distance _location _impactpoint) (Collision|BreakHitResult Hit))
  (bind _returnvalue (* _impactpoint "0.100000,0.100000,0.100000"))
  (Utilities|Casting|CastToGrippableStaticMeshActor OtherActor)
  (bind _outotherhalfprocmesh (Class|KismetProceduralMeshLibrary|SliceProceduralMesh (Variables|Default|GetProceduralMesh) _location "0, 0, 0" true "CreateNewSectionForCap"))
  (Utilities|IsValid _outotherhalfprocmesh
    (:Is%20Valid
      (Physics|SetSimulatePhysics _outotherhalfprocmesh true)
      (Physics|AddImpulse _outotherhalfprocmesh _returnvalue "None" false)
      (Physics|AddImpulse (Variables|Default|GetProceduralMesh) _returnvalue "None" false))
    (:Is%20Not%20Valid
      (Development|PrintString "Not valid"))))

(event EventBeginPlay)

(event Collision|EventActorBeginOverlap
  (params (OtherActor :type Actor%20Object%20Reference)))

(event EventTick
  (params (DeltaSeconds :type Float%20%28single-precision%29)))

(fn ConstructionScript
  (Class|KismetProceduralMeshLibrary|CopyProceduralMeshfromStaticMeshComponent (Variables|Default|GetStaticMesh) 0 (Variables|Default|GetProceduralMesh) true))