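; Base VR hammer for Whack-a-Mole, a two-handed grippable melee weapon that can lodge in objects it strikes.
; GS_Melee lodge events attach a depth-limited physics constraint, which Tick breaks on pull-out and release stiffens to hold the hammer in place.
; Grip slots snap to the GripLine spline, optionally choosing forward or reversed facing.
; Alternate-grip input slides hands along that spline, with Tick enabled for sliding or lodging.
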(event Custom|OnMeleeHit
  (params (LogComponent :type BP%20Lodge%20Component%20Info%20Structure) (OtherActor :type Actor%20Object%20Reference) (OtherComp :type Primitive%20Component%20Object%20Reference) (OtherCompCollisionChannel :type ECollisionChannel%20Enum :default "ECC_WorldStatic") (HitSurfaceProperties :type BP%20Hit%20Surface%20Properties%20Structure) (NormalImpulse :type Vector) (Hit :type Hit%20Result%20Structure%20%28by%20ref%29)))

(event Custom|LodgeEvent
  (params (LogComponent :type BP%20Lodge%20Component%20Info%20Structure) (OtherActor :type Actor%20Object%20Reference) (OtherComp :type Primitive%20Component%20Object%20Reference) (OtherCompCollisionChannel :type ECollisionChannel%20Enum :default "ECC_WorldStatic") (HitSurfaceProperties :type BP%20Hit%20Surface%20Properties%20Structure) (NormalImpulse :type Vector) (Hit :type Hit%20Result%20Structure%20%28by%20ref%29))
  (bind _returnvalue (/ (.penetrationdepth LogComponent) 2.0))
  (bind _staticmeshcomponent (Variables|Default|GetStaticMeshComponent))
  (bind _stabconstraint (Variables|Default|GetStabConstraint))
  (bind _stabconstraint_2 (Variables|Default|GetStabConstraint))
  (bind _vrgripinterfacesettings (Variables|Default|GetVRGripInterfaceSettings))
  (Utilities|IsValid (Variables|Default|GetLodgedComp)
    (:Is%20Not%20Valid
      (Variables|Default|SetLodgeDepth (.penetrationdepth LogComponent))
      (Variables|Default|SetCollisionChannel OtherCompCollisionChannel)
      (Transformation|AttachComponentToComponent _stabconstraint (.targetcomponent LogComponent) "None" "SnapToTarget" "SnapToTarget" "KeepWorld" false)
      (Transformation|SetWorldScale3D _stabconstraint "1.000000,1.000000,1.000000")
      (Class|PhysicsConstraintComponent|SetLinearXLimit _stabconstraint "LCM_Limited" _returnvalue)
      (Class|GSMelee|SetIsLodged (Variables|Default|GetMeleeScript) true OtherComp)
      (Variables|Default|SetLodgedComp OtherComp)
      (Collision|SetCollisionResponsetoChannel _staticmeshcomponent (Variables|Default|GetCollisionChannel) "ECR_Ignore")
      (Class|PhysicsConstraintComponent|SetConstrainedComponents _stabconstraint _staticmeshcomponent "None" OtherComp (.hitbonename Hit))
      (Collision|SetCollisionResponsetoChannel _staticmeshcomponent (Variables|Default|GetCollisionChannel) "ECR_Overlap")
      (bind _refframe (Class|VREPhysicsConstraintComponent|GetConstraintReferenceFrame _stabconstraint_2 "Frame1"))
      (Class|PhysicsConstraintComponent|SetConstraintReferenceFrame _stabconstraint_2 "Frame1" (Math|Transform|MakeTransform (- (.location _refframe) (* (Math|Vector|GetForwardVector (.rotation _refframe)) _returnvalue)) (.rotation _refframe) (.scale _refframe)))
      (Variables|Default|SetOriginalOnTeleport (Utilities|Struct|BreakBPInterfaceProperties _vrgripinterfacesettings))
      (Utilities|Struct|SetmembersinBPInterfaceProperties _vrgripinterfacesettings "DropOnTeleport")
      (Utilities|FlowControl|Delay 0.2)
      (Actor|Tick|SetActorTickEnabled true))))

(event Input|EnhancedActionEvents|EnhancedInputActionAlternateGripLeft
  (params (ActionValue :type Boolean) (ElapsedSeconds :type Float%20%28double-precision%29) (TriggeredSeconds :type Float%20%28double-precision%29) (InputAction :type Input%20Action%20Object%20Reference :default "/Game/VRE/Input/Actions/AlternateGripLeft.AlternateGripLeft"))
  ;[1 1 1] Slide Hands
  (:Started
    (Variables|Default|SetRepositioningLeftHand true)
    (Actor|Tick|SetActorTickEnabled (Math|Boolean|ORBoolean (Variables|Default|GetRepositioningLeftHand) (Variables|Default|GetRepositioningRightHand) (Utilities|IsValid (Variables|Default|GetLodgedComp))) :!label _label))
  (:Completed
    (Variables|Default|SetRepositioningLeftHand false)
    (goto _label)))

(event Input|EnhancedActionEvents|EnhancedInputActionAlternateGripRight
  (params (ActionValue :type Boolean) (ElapsedSeconds :type Float%20%28double-precision%29) (TriggeredSeconds :type Float%20%28double-precision%29) (InputAction :type Input%20Action%20Object%20Reference :default "/Game/VRE/Input/Actions/AlternateGripRight.AlternateGripRight"))
  ;[1 1 1] Slide Hands
  (:Started
    (Variables|Default|SetRepositioningRightHand true)
    (Actor|Tick|SetActorTickEnabled (Math|Boolean|ORBoolean (Variables|Default|GetRepositioningLeftHand) (Variables|Default|GetRepositioningRightHand) (Utilities|IsValid (Variables|Default|GetLodgedComp))) :!label _label))
  (:Completed
    (Variables|Default|SetRepositioningRightHand false)
    (goto _label)))

(event EventOnGrip
  (params (GrippingController :type Grip%20Motion%20Controller%20Component%20Object%20Reference) (GripInformation :type BP%20Actor%20Grip%20Information%20Structure%20%28by%20ref%29))
  (Input|EnableInput (Game|GetPlayerController 0))
  (Class|PhysicsConstraintComponent|SetLinearPositionTarget (Variables|Default|GetStabConstraint) (Math|Vector|MakeVector 0.0 0.0 0.0))
  (Class|PhysicsConstraintComponent|SetLinearDriveParams (Variables|Default|GetStabConstraint) 1e+03 1.5e+03 1e+03) ; This needs to be stored in a variable or somethingn instead
)

(event Collision|EventActorBeginOverlap
  (params (OtherActor :type Actor%20Object%20Reference)))

(event EventTick
  (params (DeltaSeconds :type Float%20%28single-precision%29))
  (bind _repositioninglefthand (Variables|Default|GetRepositioningLeftHand))
  (bind _gripline (Variables|Default|GetGripLine))
  (bind _meleescript (Variables|Default|GetMeleeScript))
  (bind _repositioningrighthand (Variables|Default|GetRepositioningRightHand))
  (bind _returnvalue (or _repositioninglefthand _repositioningrighthand))
  ;[1 1 1] Break Penetration
  (Utilities|FlowControl|Sequence
    (:then_0
      ;[1 1 1] Hand repositioning
      (if (Variables|Default|GetRepositioningLeftHand)
        (bind (_handpair _hadhand) (CallFunction|GetHandPair false))
        (if _hadhand
          (Class|GSMelee|UpdateHandPosition _meleescript _handpair (Spline|FindLocationClosesttoWorldLocation _gripline (Class|GripMotionControllerComponent|GetPivotLocationBP (Class|VRExpansionFunctionLibrary|ToMotionController(GripPair) _handpair)) "World")))))
    (:then_1
      (if (Variables|Default|GetRepositioningRightHand)
        (bind (_handpair_2 _hadhand_2) (CallFunction|GetHandPair true))
        (if _hadhand_2
          (Class|GSMelee|UpdateHandPositionandRotation _meleescript _handpair_2 (Math|Transform|MakeTransform (Spline|FindLocationClosesttoWorldLocation _gripline (.location (Class|GripMotionControllerComponent|GetPivotTransformBP (Class|VRExpansionFunctionLibrary|ToMotionController(GripPair) _handpair_2))) "World") (.rotation (Class|GripMotionControllerComponent|GetPivotTransformBP (Class|VRExpansionFunctionLibrary|ToMotionController(GripPair) _handpair_2))) (.scale (Class|GripMotionControllerComponent|GetPivotTransformBP (Class|VRExpansionFunctionLibrary|ToMotionController(GripPair) _handpair_2)))) true false))))
    (:then_2
      (Utilities|IsValid (Variables|Default|GetLodgedComp)
        (:Is%20Valid
          (if (<= (.x (Class|VREPhysicsConstraintComponent|GetCurrentLinearDistance (Variables|Default|GetStabConstraint) "Frame1")) (+ (/ (Variables|Default|GetLodgeDepth) -2.0) 0.501))
            (Class|PhysicsConstraintComponent|BreakConstraint (Variables|Default|GetStabConstraint))
            (Actor|Tick|SetActorTickEnabled _returnvalue)
            (Collision|SetCollisionResponsetoChannel (Variables|Default|GetStaticMeshComponent) (Variables|Default|GetCollisionChannel) "ECR_Block")
            (Variables|Default|SetLodgedComp 0)
            (Class|GSMelee|SetIsLodged (Variables|Default|GetMeleeScript) false)
            (Utilities|Struct|SetmembersinBPInterfaceProperties (Variables|Default|GetVRGripInterfaceSettings) (Variables|Default|GetOriginalOnTeleport))))
        (:Is%20Not%20Valid
          (Actor|Tick|SetActorTickEnabled _returnvalue))))))

(event EventBeginPlay
  (bind _returnvalue (Class|VRGripScriptBase|GetGripScriptbyClass "/Script/VRExpansionPlugin.GS_Melee")
    (:OnSucceeded
      (bind _asgs_melee (Utilities|Casting|CastToGS_Melee _returnvalue))
      (bind _output_get (Variables|Default|SetMeleeScript _asgs_melee))
      (EventDispatchers|BindEventtoOnShouldLodgeinObject _output_get (delegate Custom|LodgeEvent))
      (EventDispatchers|BindEventtoOnMeleeHit _output_get (delegate Custom|OnMeleeHit)))))

(event EventOnGripRelease
  (params (ReleasingController :type Grip%20Motion%20Controller%20Component%20Object%20Reference) (GripInformation :type BP%20Actor%20Grip%20Information%20Structure%20%28by%20ref%29) (bWasSocketed :type Boolean))
  (bind _stabconstraint (Variables|Default|GetStabConstraint))
  (bind _bisheld (Class|VRGripInterface|IsHeld))
  (if (not _bisheld)
    (Input|DisableInput (Game|GetPlayerController 0))
    (Utilities|IsValid (Variables|Default|GetLodgedComp)
      (:Is%20Valid
        (Class|PhysicsConstraintComponent|SetLinearPositionTarget _stabconstraint (Math|Vector|MakeVector (.x (Class|VREPhysicsConstraintComponent|GetCurrentLinearDistance _stabconstraint "Frame1")) 0.0 0.0)) ; Hold ourselves in place after grip is finished
        (Class|PhysicsConstraintComponent|SetLinearDriveParams (Variables|Default|GetStabConstraint) 1e+05 1.5e+03 1e+05)))))

(event Input|ActionEvents|InputActionAlternateGripLeft
  (params (Key :type Key%20Structure :default "None"))
  ;[1 1 1] Slide Hands
)

(event Input|ActionEvents|InputActionAlternateGripRight
  (params (Key :type Key%20Structure :default "None"))
  ;[1 1 1] Slide Hands
)

(fn ConstructionScript)

(fn ClosestGripSlotinRange
  (params (WorldLocation :type Vector :default "0, 0, 0") (bSecondarySlot :type Boolean) (CallingController :type Grip%20Motion%20Controller%20Component%20Object%20Reference) (OverridePrefix :type Name :default "None"))
  (bind _returnvalue (Transformation|GetWorldRotation CallingController))
  (bind _griprotation (Variables|Default|GetGripRotation))
  (bind _returnvalue_2 (Transformation|GetWorldRotation _griprotation))
  (LocalVariables|SetClosestSplinePoint (Spline|FindLocationClosesttoWorldLocation (Variables|Default|GetGripLine) WorldLocation "World"))
  (if (Variables|Features|GripRotation|GetUseGripRotationComponent)
    (if (Variables|Features|GripRotation|GetAutoSelectGripfacing)
      (bind (_rotation _selected_socket) (CallFunction|CalculateClosestHandRotation _returnvalue _returnvalue_2 (Transformation|GetWorldRotation (Variables|Default|GetReverseGripRotation))))
      (return true (Math|Transform|MakeTransform (LocalVariables|GetClosestSplinePoint) _rotation "1.000000,1.000000,1.000000") (Utilities|String|StringToName (Utilities|GetObjectName _selected_socket)))
      (else
        (return true (Math|Transform|MakeTransform (LocalVariables|GetClosestSplinePoint) _returnvalue_2 "1.000000,1.000000,1.000000") (Utilities|String|StringToName (Utilities|GetObjectName (Variables|Default|GetGripRotation))))))
    (else
      (return true (Math|Transform|MakeTransform (LocalVariables|GetClosestSplinePoint) _returnvalue "1.000000,1.000000,1.000000") "None"))))

(fn GetHandPair
  (params (bRightHand :type Boolean))
  (bind (_holdingcontrollers _bisheld) (Class|VRGripInterface|IsHeld))
  (if _bisheld
    (bind _array_element (Utilities|Array|ForEachLoopwithBreak _holdingcontrollers :!label _label)
      (:LoopBody
        (if (Math|Boolean|Equal(Boolean) (Utilities|Enum|Equal(Enum) (Class|GripMotionControllerComponent|GetHandType (.HoldingController (Utilities|Struct|BreakBPGripPair _array_element))) "Right") bRightHand)
          (LocalVariables|SetHandPairOut _array_element)
          (LocalVariables|SetHadValid true)
          (goto _label Break)))
      (:Completed
        (return (LocalVariables|GetHandPairOut) (LocalVariables|GetHadValid))))))

(fn CalculateClosestHandRotation
  (params (HandRotaton :type Rotator) (GripCompRotation :type Rotator) (BackwardsRotation :type Rotator))
  (bind _returnvalue (Math|Vector|GetForwardVector GripCompRotation))
  (bind _returnvalue_2 (Math|Vector|GetForwardVector HandRotaton))
  (bind _forwardgripweight (Variables|Features|GripRotation|GetForwardGripWeight))
  (bind _returnvalue_3 (Math|Vector|DotProduct _returnvalue _returnvalue_2))
  (bind _returnvalue_4 (* _forwardgripweight 1.0))
  (bind _returnvalue_5 (+ _returnvalue_3 _returnvalue_4))
  (bind _returnvalue_6 (< _returnvalue_5 0.0))
  (return (select _returnvalue_6 BackwardsRotation GripCompRotation) (select _returnvalue_6 (Variables|Default|GetReverseGripRotation) (Variables|Default|GetGripRotation))))